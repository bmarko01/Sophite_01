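; Combat component that turns light and heavy attack inputs into attack montages on a character mesh.
; Initialize caches the mesh and its anim instance for playback.
; ActionInput stores the requested move and consumes it immediately only when not attacking; otherwise it stays stored, with no later replay in this graph.
; ConsumedKey routes to LightAttack or HeavyAttack, each playing one of three montages at random.
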(event Custom|Action%20Input
  (params (Attack%20Move :type E_AttackMove%20Enum :default "NewEnumerator0"))
  (bind _output_get (Variables|Default|SetStored%20Key Attack%20Move))
  (if (not (Variables|Default|GetIsAttacking?))
    (CallFunction|ConsumedKey _output_get)
    (Variables|Default|SetStored%20Key "NewEnumerator0")))

(event Custom|Consumed%20Key
  (params (Attack%20Move :type E_AttackMove%20Enum :default "NewEnumerator0"))
  (switch Utilities|FlowControl|Switch|SwitchonE_AttackMove Attack%20Move
    (:NewEnumerator1
      (CallFunction|LightAttack))
    (:NewEnumerator2
      (CallFunction|HeavyAttack))))

(event Custom|Initialize
  (params (Mesh :type Skeletal%20Mesh%20Component%20Object%20Reference))
  (bind _output_get (Variables|Default|SetMesh Mesh))
  (Variables|Default|SetAnim%20Instance (Components|SkeletalMesh|GetAnimInstance _output_get)))

(fn LightAttack
  (Animation|Montage|MontagePlay (Variables|Default|GetAnim%20Instance) (Utilities|Array|Get(acopy) (Variables|Default|GetLAttackMontage) (Math|Random|RandomIntegerinRange 0 2)) 1.0 "MontageLength" 0.0 true))

(fn HeavyAttack
  (Animation|Montage|MontagePlay (Variables|Default|GetAnim%20Instance) (Utilities|Array|Get(acopy) (Variables|Default|GetHAttackMontage) (Math|Random|RandomIntegerinRange 0 2)) 1.0 "MontageLength" 0.0 true))