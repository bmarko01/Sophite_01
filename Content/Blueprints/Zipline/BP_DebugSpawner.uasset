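; BP_DebugSpawner is a debug actor that spawns test riders for the zipline system.
; On BeginPlay, while SpawnTests is enabled, it calls SpawnZiplineRider in a repeating Delay loop.
; Each rider is a plain StaticMeshActor spawned at the spawner's transform, given a BPC_ZiplineMovement component at runtime and set up as a movable, physics-simulated cube that generates overlap events.
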(event EventBeginPlay
  (if (Variables|Default|GetSpawnTests) :!label _label
    (CallFunction|SpawnZiplineRider)
    (Utilities|FlowControl|Delay 1.5)
    (goto _label)))

(fn ConstructionScript)

(fn SpawnZiplineRider
  (bind _returnvalue (Game|SpawnActorfromClass "/Script/Engine.StaticMeshActor" (Transformation|GetActorTransform) "Undefined" 0 0))
  (Game|AddComponentbyClass _returnvalue "/Game/Blueprints/Zipline/BPC_ZiplineMovement.BPC_ZiplineMovement_C")
  (Transformation|SetMobility (Variables|/Script/Engine.StaticMeshActor|GetStaticMeshComponent _returnvalue) "Movable")
  (Variables|/Script/Engine.PrimitiveComponent|SetbGenerateOverlapEvents (Variables|/Script/Engine.StaticMeshActor|GetStaticMeshComponent _returnvalue) true)
  (Components|StaticMesh|SetStaticMesh (Variables|/Script/Engine.StaticMeshActor|GetStaticMeshComponent _returnvalue) "/Engine/BasicShapes/Cube.Cube")
  (Physics|SetSimulatePhysics (Variables|/Script/Engine.StaticMeshActor|GetStaticMeshComponent _returnvalue) true))