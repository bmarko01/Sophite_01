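; Actor component that lets its owner attach to, detach from and change direction on ziplines, acting as a cart registered with the current zipline.
; A SwitchOwner macro branches by owner class, disabling character movement or static mesh physics on attach and restoring them on detach.
; Changing direction swaps to an alternative zipline if valid, otherwise flips ride direction.
; Tick records owner velocity, and a retriggerable delay blocks re-attachment after detaching.
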(event Custom|TimeOut_Env
  (Variables|Zipline|SetCanAttachToZipline false)
  (Utilities|FlowControl|RetriggerableDelay (Variables|Zipline,Editable|GetTimeout))
  (Variables|Zipline|SetCanAttachToZipline true))

(event EventTick
  (params (DeltaSeconds :type Float%20%28single-precision%29))
  (CallFunction|RecordOwnerVelocity DeltaSeconds))

(fn DetachfromZipline
  (Variables|Zipline|SetRidingZipline false)
  (Utilities|FlowControl|Sequence
    (:then_0
      (Utilities|SwitchOwner
        (:Sophie
          (bind _ascharacter (Utilities|Casting|CastToCharacter (Components|GetOwner) :!label _label))
          (Pawn|Components|CharacterMovement|SetMovementMode (Variables|/Script/Engine.Character|GetCharacterMovement _ascharacter) "MOVE_Falling" 0))
        (:Character
          (goto _label))
        (:StaticMesh
          (bind _asstatic_mesh_actor (Utilities|Casting|CastToStaticMeshActor (Components|GetOwner)))
          (Physics|SetSimulatePhysics (Variables|/Script/Engine.StaticMeshActor|GetStaticMeshComponent _asstatic_mesh_actor) true))))
    (:then_1
      (Utilities|IsValid (Variables|Zipline|GetCurrentZipline)
        (:Is%20Valid
          (Utilities|Array|RemoveItem (Variables|/Game/Blueprints/Zipline/BP_Zipline.BP_Zipline_C|GetAttachedCarts (Variables|Zipline|GetCurrentZipline)) self)
          (Variables|/Game/Blueprints/Zipline/BP_Zipline.BP_Zipline_C|SetConstantSpeedLerp (Variables|Zipline|GetCurrentZipline) 0.0)
          (Variables|Zipline|SetCurrentZipline 0))))
    (:then_2
      (CallFunction|TimeOutEnv))))

(fn AttachtoZipline
  (Utilities|FlowControl|Sequence
    (:then_0
      (Utilities|SwitchOwner
        (:Sophie
          (bind _ascharacter (Utilities|Casting|CastToCharacter (Components|GetOwner) :!label _label))
          (Pawn|Components|CharacterMovement|DisableMovement (Variables|/Script/Engine.Character|GetCharacterMovement _ascharacter))
          (Transformation|SetActorLocation _ascharacter (+ (Transformation|GetActorLocation _ascharacter) (Variables|Zipline,Editable|GetHangOffset)) false true))
        (:Character
          (goto _label))
        (:StaticMesh
          (bind _asstatic_mesh_actor (Utilities|Casting|CastToStaticMeshActor (Components|GetOwner)))
          (Physics|SetSimulatePhysics (Variables|/Script/Engine.StaticMeshActor|GetStaticMeshComponent _asstatic_mesh_actor) false))
        (:Default
          ;[0.05882 0.05882 0.05882] TODO if other classes need specific things to happen when attaching to a zipline put them along the respective execution flow
          (Components|Activation|SetActive (Variables|/Script/Engine.Actor|GetRootComponent (Components|GetOwner)) false false))))
    (:then_1
      (Variables|Zipline|SetRidingZipline true)
      (Variables|Zipline|SetCanAttachToZipline false))))

(fn ChangeDirection
  (Utilities|IsValid (Variables|Zipline|GetAlternativeZipline)
    (:Is%20Valid
      ;[0.05882 0.05882 0.05882] Swap ziplines if overlapping another
      (LocalVariables|SetPreviousZipline (Variables|Zipline|GetCurrentZipline))
      (CallFunction|DetachfromZipline)
      (Default|BeginAttachtoZipline (Variables|Zipline|GetAlternativeZipline) self true)
      (Variables|Zipline|SetAlternativeZipline (LocalVariables|GetPreviousZipline)))
    (:Is%20Not%20Valid
      ;[0.05882 0.05882 0.05882] Change Direction
      (Variables|Zipline|SetRideDirection (Utilities|Select :Index (Variables|Zipline|GetRideDirection) :Scroll_Down "Scroll_Up" :Scroll_Up "Scroll_Down")))))

(fn RecordOwnerVelocity
  (params (Tick :type Float%20%28single-precision%29))
  (bind _returnvalue (Components|GetOwner))
  (bind _returnvalue_2 (Transformation|GetActorLocation _returnvalue))
  (Variables|Zipline|SetOwnerVelocity (/ (Math|Vector|Distance(Vector) (Variables|Zipline|GetLastLocation) _returnvalue_2) Tick))
  (Variables|Zipline|SetLastLocation _returnvalue_2))