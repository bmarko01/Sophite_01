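; Player-placed zipline that MC_Sophie can ride.
; While Positioning, Tick traces from the owning character and camera to set both ends; PlaceZipline then stretches the cable, capsule trigger and spline between them.
; Overlap attaches Sophie to a cart at the nearest spline point, which moves either way based on the owner's facing and drops her into Falling at the end.
; Enemy overlap and invalid-placement handling are stubs.
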(event OnComponentBeginOverlap(OverlapArea)
  (params (OverlappedComponent :type Primitive%20Component%20Object%20Reference) (OtherActor :type Actor%20Object%20Reference) (OtherComp :type Primitive%20Component%20Object%20Reference) (OtherBodyIndex :type Integer) (bFromSweep :type Boolean) (SweepResult :type Hit%20Result%20Structure%20%28by%20ref%29))
  (bind _outactor (Utilities|DetermineOverlap OtherActor)
    (:Sophie
      (CallFunction|AttachtoZipline _outactor))
    (:Enemy
      ;[1 1 1] TODO put enemy damage functionality here
      (Development|PrintString "Hello"))))

(event EventBeginPlay
  (bind _ascharacter (Utilities|Casting|CastToCharacter (Components|GetOwner)))
  (Variables|Default|SetMyOwner _ascharacter))

(event EventTick
  (params (DeltaSeconds :type Float%20%28single-precision%29))
  (if (Variables|Calculations|GetPositioning)
    (Utilities|PositionEnds)
    (elif (Variables|Calculations|GetRidingZipline)
      (CallFunction|MoveCartAlongSpline)
      (if (CallFunction|IsatEndOfLine)
        (CallFunction|DetachfromZipline)))))

(fn ConstructionScript)

(fn GetStartPoint
  (bind _returnvalue (Game|GetPlayerCameraManager 0))
  (bind _myowner (Variables|Default|GetMyOwner))
  (bind _startoffset (Variables|Zipline|GetStartOffset))
  (bind _returnvalue_2 (Camera|GetCameraRotation _returnvalue))
  (bind _returnvalue_3 (Transformation|GetActorLocation _myowner))
  (bind _returnvalue_4 (Math|Rotator|MakeRotator 0.0 0.0 (.yaw _returnvalue_2)))
  (bind _returnvalue_5 (Math|Vector|RotateVector _startoffset _returnvalue_4))
  (bind _returnvalue_6 (+ _returnvalue_3 _returnvalue_5))
  (bind (_outhit _returnvalue_7) (Collision|LineTraceByChannel _returnvalue_6 (+ _returnvalue_6 (Math|Vector|MakeVector 0.0 0.0 (* (.z (.Min (Components|StaticMesh|GetLocalBounds (Variables|Default|GetStartMesh)))) 2.0))) "TraceTypeQuery1" false 0 "Persistent" true "(R=1.000000,G=0.000000,B=0.000000,A=1.000000)" "(R=0.000000,G=1.000000,B=0.000000,A=1.000000)" 2.0))
  (return _returnvalue_7 (select _returnvalue_7 (.Location (Collision|BreakHitResult _outhit)) "0, 0, 0")))

(fn PlaceZipline
  (bind _cable (Variables|Default|GetCable))
  (bind _overlaparea (Variables|Default|GetOverlapArea))
  (bind _endattach (Variables|Default|GetEndAttach))
  (bind _spline (Variables|Default|GetSpline))
  (bind _cable_2 (Variables|Default|GetCable))
  (bind _cable_3 (Variables|Default|GetCable))
  (bind _returnvalue (Transformation|GetWorldLocation _endattach))
  (bind _returnvalue_2 (Transformation|GetWorldLocation _cable))
  (Utilities|FlowControl|Sequence
    (:then_0
      (Variables|Calculations|SetPositioning false))
    (:then_1
      ;[0.03922 0.03922 0.03922] Cable Component
      (Components|Tick|SetComponentTickEnabled _cable_3 true)
      (Transformation|SetWorldScale3D _cable_3 "1.000000,1.000000,1.000000")
      (Class|CableComponent|SetAttachEndtoComponent _cable_3 (Variables|Default|GetEndAttach) "None")
      (Variables|/Script/CableComponent.CableComponent|SetCableLength _cable_2 (Math|Vector|Distance(Vector) (Transformation|GetWorldLocation _cable_2) (Transformation|GetWorldLocation (Variables|Default|GetEndAttach))))
      (Development|SetHiddeninGame _cable_3 false false))
    (:then_2
      ;[0.03922 0.03922 0.03922] Overlap Area
      (Transformation|SetWorldRotation _overlaparea (Math|Rotator|FindLookatRotation (Transformation|GetWorldLocation (Variables|Default|GetCable)) (Transformation|GetWorldLocation (Variables|Default|GetEndAttach))) false false)
      (Transformation|AddRelativeRotation _overlaparea "-90.000000, 0, 0" false false)
      (Transformation|SetWorldLocation _overlaparea (+ (/ (- _returnvalue _returnvalue_2) 2.0) _returnvalue_2) false true)
      (Components|Capsule|SetCapsuleHalfHeight _overlaparea (+ (/ (Math|Vector|Distance(Vector) _returnvalue _returnvalue_2) 2.0) (Variables|Zipline|GetWireCatchRadius)) false)
      (Components|Capsule|SetCapsuleRadius _overlaparea (Variables|Zipline|GetWireCatchRadius) true))
    (:then_3
      ;[0.03922 0.03922 0.03922] Spline
      (Transformation|SetWorldLocation _spline (Transformation|GetWorldLocation (Variables|Default|GetCable)) false true)
      (Spline|AddSplinePoint _spline (Transformation|GetWorldLocation (Variables|Default|GetEndAttach)) "World" true))))

(fn AttachtoZipline
  (params (OtherActor :type Actor%20Object%20Reference))
  (bind _spline (Variables|Default|GetSpline))
  (bind _returnvalue (Transformation|GetActorLocation OtherActor))
  (bind _returnvalue_2 (Spline|FindLocationClosesttoWorldLocation _spline _returnvalue "World"))
  (Utilities|FlowControl|Sequence
    (:then_0
      ;[0.03922 0.03922 0.03922] Position Cart along spline at overlap location
      (Transformation|SetWorldLocation (Variables|Default|GetCart) _returnvalue_2 false true)
      (Variables|Calculations|SetCurrentDistAlongSpline (Math|Vector|Distance(Vector) _returnvalue_2 (Transformation|GetWorldLocation (Variables|Default|GetSpline)))))
    (:then_1
      ;[0.03922 0.03922 0.03922] Determine ride Direction
      (Variables|Default|SetRideDirection (select (< (Math|Float|Absolute(Float) (.yaw (Math|Transform|InverseTransformRotation (Transformation|GetActorTransform (Variables|Default|GetMyOwner)) (Transformation|GetWorldRotation (Variables|Default|GetCart))))) 9e+01) "Scroll_Down" "Scroll_Up")))
    (:then_2
      ;[0.03922 0.03922 0.03922] Attach to Zipline
      (bind _output_get (Variables|Default|SetActorRidingZipline OtherActor))
      (bind _asmc_sophie (Utilities|Casting|CastToMC_Sophie _output_get))
      (Pawn|Components|CharacterMovement|DisableMovement (Variables|/Script/Engine.Character|GetCharacterMovement _asmc_sophie))
      (Transformation|AttachComponentToComponent _asmc_sophie (Variables|Default|GetCart) "None" "KeepWorld" "KeepWorld" "SnapToTarget" false)
      (Transformation|SetActorLocation _asmc_sophie (+ (Transformation|GetWorldLocation (Variables|Default|GetCart)) (Variables|Zipline|GetHangOffset)) false false))
    (:then_3
      ;[0.03922 0.03922 0.03922] Start Moving
      (Variables|Calculations|SetRidingZipline true))))

(fn DetachfromZipline
  (Variables|Calculations|SetRidingZipline false)
  (Transformation|DetachFromActor (Variables|Default|GetActorRidingZipline) "KeepWorld" "KeepWorld" "KeepWorld")
  (bind _ascharacter (Utilities|Casting|CastToCharacter (Variables|Default|GetActorRidingZipline)))
  (Pawn|Components|CharacterMovement|SetMovementMode (Variables|/Script/Engine.Character|GetCharacterMovement _ascharacter) "MOVE_Falling" 0))

(fn MoveCartAlongSpline
  (bind _returnvalue (Utilities|Time|GetWorldDeltaSeconds))
  (bind _ziplinemovespeed (Variables|Zipline|GetZiplineMoveSpeed))
  (bind _returnvalue_2 (* _ziplinemovespeed _returnvalue))
  (bind _output_get (Variables|Calculations|SetCurrentDistAlongSpline (+ (Variables|Calculations|GetCurrentDistAlongSpline) (Utilities|Select :Index (Variables|Default|GetRideDirection) :Scroll_Down _returnvalue_2 :Scroll_Up (* -1 _returnvalue_2)))))
  (Transformation|SetWorldLocation (Variables|Default|GetCart) (Spline|GetLocationatDistanceAlongSpline (Variables|Default|GetSpline) _output_get "World") false true))

(fn IsatEndOfLine
  (return (Utilities|Select :Index (Variables|Default|GetRideDirection) :Scroll_Down (>= (Variables|Calculations|GetCurrentDistAlongSpline) (Spline|GetSplineLength (Variables|Default|GetSpline))) :Scroll_Up (<= (Variables|Calculations|GetCurrentDistAlongSpline) 0.0))))